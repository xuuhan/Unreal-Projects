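; Player controller for a vehicle racing game that sets up the HUD and tracks race timing.
; On BeginPlay it adds an AnimationSampleUI widget to the viewport and stores the player's VehicleBlueprint pawn.
; Start and stop events drive GameTime and LapTime timelines, both of which write elapsed time into ActualRaceTime.
; Setup, restart, lap update, respawn and InitText are empty stubs.
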(event `self.ReceiveBeginPlay`
  ;[1 1 1] Evnet Begin Play / Get References
  ;;[1 1 1] Comment
  (bind _returnvalue (`|CreateWidget` "/DatasmithContent/Blueprints/FBXImporter/UI/AnimationSampleUI.AnimationSampleUI_C"))
  (bind _output_get (set `self.HUDReference` _returnvalue))
  (`UserWidget.AddToViewport` _output_get 0)
  (bind _asvehicle_blueprint (cast `/Game/BluePrint/VehicleBlueprint` (`GameplayStatics.GetPlayerPawn` 0)))
  (set `self.VehicleReference` _asvehicle_blueprint))

(event `StarGameSetup`)

(event `StartRaceTime`
  (bind (_direction _time) (`Timeline|GameTime` :!label _label)
    (:`Update`
      (set `self.ActualRaceTime` _time))))

(event `StopRaceTime`
  (goto _label :!via `Stop`))

(event `Restart`)

(event `StartLapTime`
  (bind (_direction _time) (`Timeline|LapTime` :!via `PlayFromStart` :!label _label_2)
    (:`Update`
      (set `self.ActualRaceTime` _time))))

(event `UpdateLap`)

(event `StopLapTime`
  (goto _label_2 :!via `Stop`))

(event `RespawnVehicle`)

(fn `InitText`)

(fn `UserConstructionScript`)