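; TimeConversion is a Blueprint with a TimeToText graph meant to format a time value as minutes:seconds.hundredths text; its construction script is empty.
; The formatting chain is marked unused, so it drives no output.
; It joins floored fields with separators, but the seconds field repeats the minutes calculation.
; Its zero-padding is inverted, prefixing "0" to values of 9 or more instead of single digits.
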(fn `UserConstructionScript`)