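; A player controller for a racing game that creates the HUD and tracks race time.
; BeginPlay adds the HUD, caches the player's VehicleBlueprint pawn and starts the race timer.
; GameTime and LapTime timelines act as stopwatches, both writing ActualRaceTime, with race time also converted to text and printed.
; InitText converts lap values to text, while setup, restart, respawn, lap update and lap check are empty stubs.
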(event `self.ReceiveBeginPlay`
  ;[1 1 1] Evnet Begin Play / Get References
  ;;[1 1 1] Comment
  (bind _returnvalue (`|CreateWidget` "/Game/BluePrints/UI/HUD.HUD_C"))
  (bind _output_get (set `self.HUDReference` _returnvalue))
  (`UserWidget.AddToViewport` _output_get 0)
  (bind _asvehicle_blueprint (cast `/Game/BluePrints/VehicleBlueprint` (`GameplayStatics.GetPlayerPawn` 0))
    (:`then`
      (set `self.VehicleReference` _asvehicle_blueprint)
      (`self.StartRaceTime`))
    (:`CastFailed`
      (`KismetSystemLibrary.PrintString` "error!~"))))

(event `StarGameSetup`)

(event `StartRaceTime`
  ;[1 1 1] Race / Lap Time
  (bind (_direction _time) (`Timeline|GameTime` :!label _label)
    (:`Update`
      (bind _output_get (set `self.ActualRaceTime` _time))
      (bind _output_get_2 (set `self.RaceTimeText` (`/Game/BluePrints/TimeConversion.TimeToText` _output_get)))
      (`KismetSystemLibrary.PrintString` (`KismetTextLibrary.Conv_TextToString` _output_get_2)))))

(event `StopRaceTime`
  ;[1 1 1] Race / Lap Time
  (goto _label :!via `Stop`))

(event `Restart`)

(event `StartLapTime`
  ;[1 1 1] Race / Lap Time
  (bind (_direction _time) (`Timeline|LapTime` :!via `PlayFromStart` :!label _label_2)
    (:`Update`
      (set `self.ActualRaceTime` _time))))

(event `UpdateLap`)

(event `StopLapTime`
  ;[1 1 1] Race / Lap Time
  (goto _label_2 :!via `Stop`))

(event `RespawnVehicle`)

(fn `InitText`
  ;[1 1 1] GameText
  (set `self.CurrentLapText` (`KismetTextLibrary.Conv_IntToText` (`self.ActualLap`)))
  (set `self.MaxLapText` (`KismetTextLibrary.Conv_IntToText` (`self.MaxLaps`)))
  (set `self.BestLapText` (`KismetTextLibrary.Conv_IntToText` (`self.BestLapTime`))))

(fn `LapTimeCheck`)

(fn `UserConstructionScript`)